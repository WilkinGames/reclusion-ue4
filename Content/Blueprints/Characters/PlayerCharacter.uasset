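; Player character Blueprint that sets up the game HUD and lets the player spawn mutant enemies on demand.
; BeginPlay creates the HUD and caches its crosshair widget, which Tick hides while aiming and otherwise feeds the current spread.
; Tab traces along the control rotation and spawns a MutantCharacter with a default controller, slightly above the hit point or at the trace's end if nothing is hit.
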(event EventBeginPlay
  (bind _returnvalue (UserInterface|CreateWidget "/Game/UserInterface/UMG/Widgets/GameHUD.GameHUD_C" (Game|GetPlayerController 0)))
  (Variables|Default|SetGameHUDWidget _returnvalue)
  (Variables|Default|SetCrosshairWidget (Variables|/Game/UserInterface/UMG/Widgets/GameHUD.GameHUD_C|GetCrosshair _returnvalue))
  (UserInterface|Viewport|AddtoViewport _returnvalue))

(event EventTick
  (params (DeltaSeconds :type Float%20%28single-precision%29))
  (if (Class|ReclusionCharacter|IsAiming)
    (Widget|SetVisibility (Variables|Default|GetCrosshairWidget) "Hidden")
    (else
      (Widget|SetVisibility (Variables|Default|GetCrosshairWidget) "Visible")
      (Variables|/Game/UserInterface/UMG/Widgets/Crosshair.Crosshair_C|Setcrosshair_spread (Variables|Default|GetCrosshairWidget) (Variables|Default|GetCrosshairSpread)))))

(event Input|KeyboardEvents|Tab
  (bind _returnvalue (Transformation|GetActorLocation))
  (bind _returnvalue_2 (Pawn|GetControlRotation :!class /Script/Engine.Pawn))
  (bind _returnvalue_3 (Math|Vector|RotateVector "3000.000000,0.000000, 0" _returnvalue_2))
  (bind _returnvalue_4 (+ _returnvalue _returnvalue_3))
  (:Pressed
    (bind (_outhit _returnvalue_5) (Collision|LineTraceByChannel 0 (Transformation|GetActorLocation) _returnvalue_4 "TraceTypeQuery1" false 0 "None"))
    (if _returnvalue_5
      (Variables|Default|SetMutantSpawnTransform (Math|Conversions|ToTransform(Vector) (+ (.Location (Collision|BreakHitResult _outhit)) "0, 0,96.000000")))
      (else
        (Variables|Default|SetMutantSpawnTransform (Math|Conversions|ToTransform(Vector) _returnvalue_4))))
    (bind _returnvalue_6 (Game|SpawnActorfromClass "/Game/Blueprints/Characters/MutantCharacter.MutantCharacter_C" (Variables|Default|GetMutantSpawnTransform) false 0))
    (Pawn|SpawnDefaultController _returnvalue_6)))

(fn ConstructionScript)